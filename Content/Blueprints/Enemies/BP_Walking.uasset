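; BP_Walking is an enemy that walks a looping patrol path, fires twin guns and damages the VR player on contact.
; Tick moves EnemyOffset in relative space at constant speed toward the current point, easing rotation toward travel direction.
; A looping timer fires both guns, spawning projectiles with animation and sound, without aiming or target checks.
; Death extends the parent with an explosion and sound at the head.
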(event OnComponentBeginOverlap(Box)
  (params (OverlappedComponent :type Primitive%20Component%20Object%20Reference) (OtherActor :type Actor%20Object%20Reference) (OtherComp :type Primitive%20Component%20Object%20Reference) (OtherBodyIndex :type Integer) (bFromSweep :type Boolean) (SweepResult :type Hit%20Result%20Structure%20%28by%20ref%29))
  (bind _asvrpawn (Utilities|Casting|CastToVRPawn OtherActor))
  (Game|Damage|ApplyDamage _asvrpawn 1e+01 0 self))

(event Custom|Fire
  ;[1 1 1] SHot
  (Utilities|FlowControl|Sequence
    (:then_0
      (CallFunction|FireGun (Variables|Default|GetSK_CSC_Gun1) (Variables|Default|GetFireLeft))
      (CallFunction|FireGun (Variables|Default|GetSK_CSC_Gun2) (Variables|Default|GetFireRight)))))

(event Custom|FireGun
  (params (GunMesh :type Skeletal%20Mesh%20Component%20Object%20Reference) (FirePoint :type Scene%20Component%20Object%20Reference))
  (bind _returnvalue (Transformation|GetWorldLocation FirePoint))
  ;[1 1 1] SHot
  (Components|Animation|PlayAnimation GunMesh "/Game/Meshes/Ennemies/Animations/Anim_CSC_Gun1.Anim_CSC_Gun1" false)
  (Game|SpawnActorfromClass "/Game/Blueprints/BP_EnnemyProjectile.BP_EnnemyProjectile_C" (Math|Transform|MakeTransform _returnvalue (Transformation|GetWorldRotation FirePoint) "1,1,1") "Undefined" 0 0)
  (Audio|PlaySoundatLocation "/Game/Meshes/Ennemies/Demo/Sounds/LaserShot.LaserShot" _returnvalue "0, 0, 0" 0.75 1.0 0.0 "/Game/Audio/AttenuationSettings/FireAttenuation.FireAttenuation" 0 0))

(event EventTick
  (params (DeltaSeconds :type Float%20%28single-precision%29))
  (bind _enemyoffset (Variables|Default|GetEnemyOffset))
  (bind _enemyoffset_2 (Variables|Default|GetEnemyOffset))
  (bind _relativelocation (Variables|/Script/Engine.SceneComponent|GetRelativeLocation _enemyoffset_2))
  (Utilities|FlowControl|Sequence
    (:then_0
      (Transformation|SetRelativeRotation _enemyoffset (Math|Interpolation|RInterpTo (Variables|/Script/Engine.SceneComponent|GetRelativeRotation (Variables|Default|GetEnemyOffset)) (Math|Conversions|RotationFromXVector (Math|Vector|Normalize (- (Math|Interpolation|VInterptoConstant _relativelocation (Utilities|Array|Get(acopy) (Variables|Default|GetPatrolPath) (Variables|Default|GetCurrentPathPoint)) (Utilities|Time|GetWorldDeltaSeconds) (Variables|Default|GetSpeed)) _relativelocation))) (Utilities|Time|GetWorldDeltaSeconds) 1e+01) false false)
      (Transformation|SetRelativeLocation _enemyoffset (Math|Interpolation|VInterptoConstant _relativelocation (Utilities|Array|Get(acopy) (Variables|Default|GetPatrolPath) (Variables|Default|GetCurrentPathPoint)) (Utilities|Time|GetWorldDeltaSeconds) (Variables|Default|GetSpeed)) false false))
    (:then_1
      (if (< (Class|KismetMathLibrary|VectorDistanceSquared (Variables|/Script/Engine.SceneComponent|GetRelativeLocation (Variables|Default|GetEnemyOffset)) (Utilities|Array|Get(acopy) (Variables|Default|GetPatrolPath) (Variables|Default|GetCurrentPathPoint))) 1e+01)
        (Variables|Default|SetCurrentPathPoint (Math|Integer|%(Integer) (+ (Variables|Default|GetCurrentPathPoint) 1) (Utilities|Array|Length (Variables|Default|GetPatrolPath))))))))

(event EventBeginPlay
  ;[1 1 1] SHot
  (Utilities|Time|SetTimerbyEvent (delegate Custom|Fire) 1.0 true)
  (Transformation|SetRelativeLocation (Variables|Default|GetEnemyOffset) (Utilities|Array|Get(acopy) (Variables|Default|GetPatrolPath)) false false))

(fn ConstructionScript)

(fn Death
  (bind _sk_rlv_head (Variables|Default|GetSK_RLV_head))
  (bind _returnvalue (Transformation|GetWorldLocation _sk_rlv_head))
  (|CallParentFunction)
  (Effects|SpawnEmitteratLocation "/Game/Meshes/Ennemies/Demo/Particles/P_Explosion.P_Explosion" _returnvalue)
  (Audio|PlaySoundatLocation "/Game/Meshes/Ennemies/Demo/Sounds/unitDead.unitDead" _returnvalue "0, 0, 0" 1.0 1.0 0.0 "/Game/Audio/AttenuationSettings/FireAttenuation.FireAttenuation" 0 0))