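; Enemy tower that spins its gun assembly while alive and fires without aiming, in a game with a VR pawn.
; A looping timer fires both left and right guns together, each playing an animation and sound and spawning an enemy projectile from its muzzle socket.
; A box overlap damages the VRPawn on contact.
; Death extends the parent's logic with an explosion effect and sound; firing itself has no life check.
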(event OnComponentBeginOverlap(Box)
  (params (OverlappedComponent :type Primitive%20Component%20Object%20Reference) (OtherActor :type Actor%20Object%20Reference) (OtherComp :type Primitive%20Component%20Object%20Reference) (OtherBodyIndex :type Integer) (bFromSweep :type Boolean) (SweepResult :type Hit%20Result%20Structure%20%28by%20ref%29))
  (bind _asvrpawn (Utilities|Casting|CastToVRPawn OtherActor))
  (Game|Damage|ApplyDamage _asvrpawn 1e+01 0 self))

(event Custom|Fire
  ;[1 1 1] SHot
  (Utilities|FlowControl|Sequence
    (:then_0
      (Variables|Default|SetskeletWeap (Variables|Default|GetSK_CSC_gunL)))
    (:then_1
      (Variables|Default|SetskeletWeap (Variables|Default|GetSK_CSC_gunR))))
  (Components|Animation|PlayAnimation (Variables|Default|GetskeletWeap) "/Game/Meshes/Ennemies/Animations/Anim_CSC_Gun3.Anim_CSC_Gun3" false)
  (Game|SpawnActorfromClass "/Game/Blueprints/BP_EnnemyProjectile.BP_EnnemyProjectile_C" (Math|Transform|MakeTransform (Transformation|GetSocketLocation (Variables|Default|GetskeletWeap) "Gun_EndSocket") (Transformation|GetSocketRotation (Variables|Default|GetskeletWeap) "Gun_EndSocket") "1,1,1") "Undefined" 0 0)
  (Audio|PlaySoundatLocation "/Game/Meshes/Ennemies/Demo/Sounds/LaserShot.LaserShot" (Transformation|GetSocketLocation (Variables|Default|GetskeletWeap) "Gun_EndSocket") "0, 0, 0" 1.5 1.0 0.0 "/Game/Audio/AttenuationSettings/FireAttenuation.FireAttenuation" 0 0))

(event EventTick
  (params (DeltaSeconds :type Float%20%28single-precision%29))
  (if (> (Variables|Default|GetLifeStat) 0.0)
    (Transformation|AddLocalRotation (Variables|Default|GetSK_CSC_Gun6) (Math|Rotator|MakeRotator 0.0 0.0 (* DeltaSeconds 9e+01)) false false)))

(event EventBeginPlay
  ;[1 1 1] SHot
  (Utilities|Time|SetTimerbyEvent (delegate Custom|Fire) 0.5 true))

(fn ConstructionScript)

(fn Death
  (bind _sk_csc_gun6 (Variables|Default|GetSK_CSC_Gun6))
  (bind _returnvalue (Transformation|GetWorldLocation _sk_csc_gun6))
  (|CallParentFunction)
  (Effects|SpawnEmitteratLocation "/Game/Meshes/Ennemies/Demo/Particles/P_Explosion.P_Explosion" _returnvalue)
  (Audio|PlaySoundatLocation "/Game/Meshes/Ennemies/Demo/Sounds/unitDead.unitDead" _returnvalue "0, 0, 0" 1.0 1.0 0.0 "/Game/Audio/AttenuationSettings/FireAttenuation.FireAttenuation" 0 0))