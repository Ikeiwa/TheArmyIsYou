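; VR ghost actor that replays recorded player movement and weapon fire from GhostData, restarting when the recording ends.
; On BeginPlay it spawns the recorded weapon class, if valid, and grabs it with the recorded hand.
; Tick interpolates actor position plus head and hand transforms between timestamped frames, advancing at most one frame per tick.
; Changes in the recorded fire state send trigger pressed or released messages to the held weapon.
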(event Custom|StopFire
  ;[0.03434 0.03434 0.03434] InputAction Trigger Left/Right
  (bind _heldcomponent (Variables|Default|GetHeldComponent)
    (:then
      (Class|VRInteractionBPI|TriggerReleased(Message) (Components|GetOwner _heldcomponent)))
    (:else)))

(event Custom|Fire
  ;[0.03434 0.03434 0.03434] InputAction Trigger Left/Right
  (bind _heldcomponent (Variables|Default|GetHeldComponent)
    (:then
      (Class|VRInteractionBPI|TriggerPressed(Message) (Components|GetOwner _heldcomponent)))
    (:else)))

(event Custom|StartPlayback
  (Variables|Default|SetSpawnTime (Actor|GetGameTimeSinceCreation))
  (Variables|Default|SetCurrentFrame 0))

(event EventBeginPlay
  (bind _ghostdata (Variables|Default|GetGhostData))
  (bind (_weapon _righthand) (Utilities|Struct|BreakGhostData _ghostdata))
  (CallFunction|StartPlayback)
  (if (Utilities|IsValidClass _weapon)
    (bind _returnvalue (Game|SpawnActorfromClass _weapon (Math|Transform|MakeTransform "0, 0, 0") "AlwaysSpawn" 0 self))
    (Default|TryGrab (Actor|GetComponentbyClass _returnvalue "/Game/Blueprints/GrabComponent.GrabComponent_C") (select _righthand (Variables|Default|GetRightHand) (Variables|Default|GetLeftHand)))
    (Variables|Default|SetHeldComponent (Actor|GetComponentbyClass _returnvalue "/Game/Blueprints/GrabComponent.GrabComponent_C"))))

(event EventTick
  (params (DeltaSeconds :type Float%20%28single-precision%29))
  (bind _returnvalue (Actor|GetGameTimeSinceCreation))
  (bind _spawntime (Variables|Default|GetSpawnTime))
  (bind _ghostdata (Variables|Default|GetGhostData))
  (bind _currentframe (Variables|Default|GetCurrentFrame))
  (bind _ghostdata_2 (Variables|Default|GetGhostData))
  (bind _currentframe_2 (Variables|Default|GetCurrentFrame))
  (bind _currentframe_3 (Variables|Default|GetCurrentFrame))
  (bind _times (Utilities|Struct|BreakGhostData _ghostdata))
  (bind (_position _headposition _headrotation _lefthandposition _lefthandrotation _righthandposition _righthandrotation _fire) (Utilities|Struct|BreakGhostData _ghostdata_2))
  (bind _returnvalue_2 (- _returnvalue _spawntime))
  (bind _returnvalue_3 (+ _currentframe 1))
  (bind _returnvalue_4 (+ _currentframe_2 1))
  (bind _output (Utilities|Array|Get(acopy) _times _returnvalue_3))
  (bind _output_2 (Utilities|Array|Get(acopy) _times _currentframe))
  (bind _output_3 (Utilities|Array|Get(acopy) _fire _currentframe_3))
  (bind _returnvalue_5 (- _output _output_2))
  (bind _returnvalue_6 (- _returnvalue_2 _output_2))
  (bind _returnvalue_7 (/ _returnvalue_6 _returnvalue_5))
  (if (< (Variables|Default|GetCurrentFrame) (- (Utilities|Array|Length (Utilities|Struct|BreakGhostData (Variables|Default|GetGhostData))) 2))
    (Utilities|FlowControl|Sequence
      (:then_0
        (Transformation|SetActorLocation (Math|Vector|Lerp(Vector) (Utilities|Array|Get(acopy) _position _currentframe_3) (Utilities|Array|Get(acopy) _position _returnvalue_4) _returnvalue_7) false false)
        (Transformation|SetWorldLocationAndRotation (Variables|Default|GetHead) (Math|Vector|Lerp(Vector) (Utilities|Array|Get(acopy) _headposition _currentframe_3) (Utilities|Array|Get(acopy) _headposition _returnvalue_4) _returnvalue_7) (Math|Rotator|Lerp(Rotator) (Utilities|Array|Get(acopy) _headrotation _currentframe_3) (Utilities|Array|Get(acopy) _headrotation _returnvalue_4) _returnvalue_7 true) false false)
        (Transformation|SetWorldLocationAndRotation (Variables|Default|GetLeftHand) (Math|Vector|Lerp(Vector) (Utilities|Array|Get(acopy) _lefthandposition _currentframe_3) (Utilities|Array|Get(acopy) _lefthandposition _returnvalue_4) _returnvalue_7) (Math|Rotator|Lerp(Rotator) (Utilities|Array|Get(acopy) _lefthandrotation _currentframe_3) (Utilities|Array|Get(acopy) _lefthandrotation _returnvalue_4) _returnvalue_7 true) false false)
        (Transformation|SetWorldLocationAndRotation (Variables|Default|GetRightHand) (Math|Vector|Lerp(Vector) (Utilities|Array|Get(acopy) _righthandposition _currentframe_3) (Utilities|Array|Get(acopy) _righthandposition _returnvalue_4) _returnvalue_7) (Math|Rotator|Lerp(Rotator) (Utilities|Array|Get(acopy) _righthandrotation _currentframe_3) (Utilities|Array|Get(acopy) _righthandrotation _returnvalue_4) _returnvalue_7 true) false false)
        (if (Math|Boolean|NotEqual(Boolean) _output_3 (Variables|Default|GetLastFire))
          (bind _output_get (Variables|Default|SetLastFire _output_3))
          (if _output_get
            (CallFunction|Fire)
            (else
              (CallFunction|StopFire)))))
      (:then_1
        (if (or (>= _returnvalue_7 1.0) (== _output_2 _output))
          (Math|Integer|IncrementInt (Variables|Default|GetCurrentFrame)))))
    (else
      (CallFunction|StartPlayback)
      (Development|PrintString "Recording Ended"))))

(fn ConstructionScript)